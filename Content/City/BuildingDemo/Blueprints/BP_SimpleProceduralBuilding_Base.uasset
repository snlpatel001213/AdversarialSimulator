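; BP_SimpleProceduralBuilding_Base is a base Blueprint for a simple procedural building made by scaling a single mesh.
; SetSize scales the mesh by depth, width and floor count, each multiplied by a unit conversion factor.
; With RandomOnMove set, the construction script first picks truncated random dimensions within configurable ranges, re-rolling whenever it reruns, such as on an editor move.
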(event Custom|RandomSize
  (bind _depthrange (Variables|Setup-Random|GetDepthRange))
  (bind _widthrange (Variables|Setup-Random|GetWidthRange))
  (bind _floorrange (Variables|Setup-Random|GetFloorRange))
  (Variables|Setup|SetDepth (Math|Float|Truncate (Math|Random|RandomFloatinRange (.x _depthrange) (.y _depthrange))))
  (Variables|Setup|SetWidth (Math|Float|Truncate (Math|Random|RandomFloatinRange (.x _widthrange) (.y _widthrange))))
  (Variables|Setup|SetNumberOfFloors (Math|Float|Truncate (Math|Random|RandomFloatinRange (.x _floorrange) (.y _floorrange))))
  (CallFunction|SetSize))

(event Custom|SetSize
  (Transformation|SetWorldScale3D (Variables|Default|GetMesh) (Math|Vector|MakeVector (* (Variables|Setup|GetDepth) (Variables|Default|GetUnitConversion)) (* (Variables|Setup|GetWidth) (Variables|Default|GetUnitConversion)) (* (Variables|Setup|GetNumberOfFloors) (Variables|Default|GetUnitConversion)))))

(fn ConstructionScript
  (if (Variables|Setup-Random|GetRandomOnMove?)
    (CallFunction|RandomSize)
    (else
      (CallFunction|SetSize))))